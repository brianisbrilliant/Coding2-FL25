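; BP_ScaredEnemy is an AI enemy that continually flees from the player character.
; On BeginPlay it caches the player and starts RunAway, which moves to a random reachable point around a spot 500 units directly away from the player.
; RunAway re-triggers itself whether the move succeeds or fails, with no distance check.
; A separate EDamage event reduces Health and destroys the actor at zero or below.
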(event Custom|RunAway
  (bind _returnvalue (Transformation|GetActorLocation))
  (bind _charref (Variables|Default|GetCharRef))
  (bind _returnvalue_2 (Transformation|GetActorLocation _charref))
  (bind _returnvalue_3 (Math|Rotator|FindLookatRotation _returnvalue _returnvalue_2))
  (bind _returnvalue_4 (Math|Vector|GetForwardVector _returnvalue_3))
  (bind _returnvalue_5 (* _returnvalue_4 -5e+02))
  (bind _returnvalue_6 (+ _returnvalue _returnvalue_5))
  (bind (_x _y) (Math|Vector|BreakVector _returnvalue_6))
  (AI|AIMoveTo self (.RandomLocation (AI|Navigation|GetRandomReachablePointinRadius (Math|Vector|MakeVector _x _y (.Z (Math|Vector|BreakVector _returnvalue))) 5e+02 0 0)) 0 5.0 false
    (:OnSuccess
      _)
    (:OnFail
      _))
  (CallFunction|RunAway))

(event EventBeginPlay
  (bind _asbp_third_person_character (Utilities|Casting|CastToBP_ThirdPersonCharacter (Game|GetPlayerCharacter 0)))
  (Variables|Default|SetCharRef _asbp_third_person_character)
  (CallFunction|RunAway))

(event EventEDamage
  (params (Damage :type Float%20%28double-precision%29))
  (bind _output_get (Variables|Default|SetHealth (- (Variables|Default|GetHealth) Damage)))
  (if (<= _output_get 0.0)
    (Actor|DestroyActor)))

(fn ConstructionScript)