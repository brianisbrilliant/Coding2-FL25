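; Boomerang item that the player holds in the right hand and throws to damage actors tagged Enemy.
; UsePrimary clears the character's held item, drops it and starts a spinning, swept flight with a whoosh sound.
; Each tick, a falling Force scales movement along the live camera forward, reversing it once negative, unless PlayerCheck is set.
; Box overlaps deal damage; the saved throw direction and look-at return move are unused.
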(event OnComponentBeginOverlap(Box)
  (params (OverlappedComponent :type Primitive%20Component%20Object%20Reference) (OtherActor :type Actor%20Object%20Reference) (OtherComp :type Primitive%20Component%20Object%20Reference) (OtherBodyIndex :type Integer) (bFromSweep :type Boolean) (SweepResult :type Hit%20Result%20Structure%20%28by%20ref%29))
  (if (Actor|ActorHasTag OtherActor "Enemy")
    (Development|PrintString "maybenifndms")
    (Class|BPIDamage|EDamage(Message) OtherActor 5e+01)))

(event EventTick
  (params (DeltaSeconds :type Float%20%28single-precision%29))
  (bind _returnvalue (Transformation|GetActorRotation))
  (if (Variables|Default|GetThrown)
    (Variables|Default|SetForce (- (Variables|Default|GetForce) 0.5))
    (if (not (Variables|Default|GetPlayerCheck))
      (Transformation|SetActorLocationAndRotation (+ (Transformation|GetActorLocation) (* (Transformation|GetActorForwardVector (Game|GetPlayerCameraManager 0)) (Variables|Default|GetForce))) (Math|Rotator|MakeRotator (.roll _returnvalue) (.pitch _returnvalue) (+ (.yaw _returnvalue) 1e+01)) true))))

(event EventUsePrimary
  (bind _asbp_third_person_character (Utilities|Casting|CastToBP_ThirdPersonCharacter (Game|GetPlayerCharacter 0)))
  (Variables|/Game/ThirdPerson/Blueprints/BP_ThirdPersonCharacter.BP_ThirdPersonCharacter_C|SetHeldItem _asbp_third_person_character 0)
  (Class|BPIItemm|Drop(Message) self)
  (Variables|Default|SetThrown true)
  (Variables|Default|Setcamforward (Transformation|GetActorForwardVector (Game|GetPlayerCameraManager 0)))
  (Audio|SpawnSoundAttached "/Game/Sound/spin-whoosh-1-186596.spin-whoosh-1-186596" (Variables|Default|GetSphere) "None" "0, 0, 0" "0, 0, 0" "KeepRelativeOffset" false 1.0 1.0 0.0 0 0))

(event EventPickup
  (params (SkeletalMesh :type Skeletal%20Mesh%20Component%20Object%20Reference))
  (Transformation|AttachComponentToComponent SkeletalMesh "hand_r" "SnapToTarget" "KeepWorld" "KeepRelative" true)
  (Collision|SetCollisionEnabled (Variables|Default|GetBox1) "NoCollision")
  (Variables|Default|SetThrown false))

(event EventDrop
  (Transformation|DetachFromActor "KeepWorld" "KeepWorld" "KeepWorld")
  (Collision|SetCollisionEnabled (Variables|Default|GetBox1) "QueryAndPhysics"))

(fn ConstructionScript)