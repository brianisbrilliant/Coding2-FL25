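; BP_Bullet is a projectile actor that flies straight along its forward vector and damages the player on contact.
; Each Tick moves it a fixed step forward with a swept SetActorLocation, so speed depends on frame rate rather than delta time.
; A Sphere overlap calls PDamageMessage on the player character with fixed damage, then destroys the bullet on any overlap.
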(event OnComponentBeginOverlap(Sphere)
  (params (OverlappedComponent :type Primitive%20Component%20Object%20Reference) (OtherActor :type Actor%20Object%20Reference) (OtherComp :type Primitive%20Component%20Object%20Reference) (OtherBodyIndex :type Integer) (bFromSweep :type Boolean) (SweepResult :type Hit%20Result%20Structure%20%28by%20ref%29))
  (if (== OtherActor (Game|GetPlayerCharacter 0))
    (Class|BPIDamage|PDamage(Message) OtherActor 5e+01))
  (Actor|DestroyActor))

(event EventTick
  (params (DeltaSeconds :type Float%20%28single-precision%29))
  (Transformation|SetActorLocation (+ (Transformation|GetActorLocation) (* (Transformation|GetActorForwardVector) 1e+01)) true false))

(fn ConstructionScript)