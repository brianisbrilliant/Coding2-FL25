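; BP_ElementalBarrier is a barrier of one element that kills a player character lacking immunity to it.
; On BeginPlay it labels its TextRender with a name chosen from its ElementalType.
; When BP_ThirdPersonCharacter overlaps the Cube, a mismatch between ElementalType and the character's ElementalImmunity prints a death message and quits the game after a short delay.
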(event OnComponentBeginOverlap(Cube)
  (params (OverlappedComponent :type Primitive%20Component%20Object%20Reference) (OtherActor :type Actor%20Object%20Reference) (OtherComp :type Primitive%20Component%20Object%20Reference) (OtherBodyIndex :type Integer) (bFromSweep :type Boolean) (SweepResult :type Hit%20Result%20Structure%20%28by%20ref%29))
  (bind _asbp_third_person_character (Utilities|Casting|CastToBP_ThirdPersonCharacter OtherActor))
  (if (not (Utilities|Enum|Equal(Enum) (Variables|Default|GetElemental%20Type) (Variables|/Game/ThirdPerson/Blueprints/BP_ThirdPersonCharacter.BP_ThirdPersonCharacter_C|GetElemental%20Immunity _asbp_third_person_character)))
    (Development|PrintText "You're dead!")
    (Utilities|FlowControl|Delay 2.0)
    (Game|QuitGame 0 "Quit" false)))

(event EventBeginPlay
  (Development|PrintText (|GenerictoText (Variables|Default|GetElemental%20Type)))
  (switch Utilities|FlowControl|Switch|SwitchonElementalType (Variables|Default|GetElemental%20Type)
    (:NewEnumerator1
      (Rendering|Components|TextRender|SetText (Variables|Default|GetTextRender) (Utilities|Text|MakeLiteralText "Barrier of Fire")))
    (:NewEnumerator2
      (Rendering|Components|TextRender|SetText (Variables|Default|GetTextRender) (Utilities|Text|MakeLiteralText "Barrier of Ice")))
    (:NewEnumerator3
      (Rendering|Components|TextRender|SetText (Variables|Default|GetTextRender) (Utilities|Text|MakeLiteralText "Barrier of Stone")))
    (:NewEnumerator4
      (Rendering|Components|TextRender|SetText (Variables|Default|GetTextRender) (Utilities|Text|MakeLiteralText "Barrier of Wind")))
    (:NewEnumerator5
      (Rendering|Components|TextRender|SetText (Variables|Default|GetTextRender) (Utilities|Text|MakeLiteralText "Barrier of Acid")))
    (:NewEnumerator6
      (Rendering|Components|TextRender|SetText (Variables|Default|GetTextRender) (Utilities|Text|MakeLiteralText "Barrier of Darkness")))))

(fn ConstructionScript)