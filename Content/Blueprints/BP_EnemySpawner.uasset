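; BP_EnemySpawner populates the level with AI enemies when play begins.
; It finds every BPEnemySpawnPoint actor and, with a weighted random chance at each, spawns a BP_AiMoveTo at that point's transform.
; Each spawned enemy gets a fixed name on its text render component, the Manny skeletal mesh and pink and blue flat materials.
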(event EventBeginPlay
  (Development|PrintString "enemy spawner is active")
  (bind _outactors (Actor|GetAllActorsOfClass "/Game/Blueprints/BPEnemySpawnPoint.BPEnemySpawnPoint_C"))
  (for _array_element _outactors
    (if (Math|Random|RandomBoolwithWeight 0.75)
      (bind _returnvalue (Game|SpawnActorfromClass "/Game/AI_Blueprints/BP_AiMoveTo.BP_AiMoveTo_C" (Transformation|GetActorTransform _array_element) "Undefined" "MultiplyWithRoot" 0 0)) ; Spawn actor from class
      (Rendering|Components|TextRender|SetText (Variables|/Game/AI_Blueprints/BP_AiMoveTo.BP_AiMoveTo_C|GetAI%20Name%20Text _returnvalue) (Utilities|Text|MakeLiteralText "Chewbacca")) ; Use an array to specify a random name.
      (Components|SkeletalMesh|SetSkeletalMeshAsset (Variables|/Script/Engine.Character|GetMesh _returnvalue) "/Game/Characters/Mannequins/Meshes/SKM_Manny.SKM_Manny")
      (Rendering|Material|SetMaterial (Variables|/Script/Engine.Character|GetMesh _returnvalue) 0 "/Game/Materials/MI_FlatPink.MI_FlatPink")
      (Rendering|Material|SetMaterial (Variables|/Script/Engine.Character|GetMesh _returnvalue) 1 "/Game/Materials/MI_FlatBlue.MI_FlatBlue"))))

(fn ConstructionScript)