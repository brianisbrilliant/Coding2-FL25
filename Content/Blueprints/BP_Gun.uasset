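; BP_Gun is a gun that can be picked up, dropped and fired.
; UsePrimary spawns a BP_PlayerBullet at the Scene component's location, using the first player's camera rotation so shots follow the view direction.
; Pickup attaches the gun to the given skeletal mesh's hand_r socket, keeping world rotation, and disables Box collision.
; Drop detaches it in place and restores query and physics collision.
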(event EventUsePrimary
  (Game|SpawnActorfromClass "/Game/Blueprints/BP_PlayerBullet.BP_PlayerBullet_C" (Math|Transform|MakeTransform (Transformation|GetWorldLocation (Variables|Default|GetScene)) (Transformation|GetActorRotation (Game|GetPlayerCameraManager 0)) "1.000000,1.000000,1.000000") "Undefined" "MultiplyWithRoot" 0 0))

(event EventPickup
  (params (SkeletalMesh :type Skeletal%20Mesh%20Component%20Object%20Reference))
  (Transformation|AttachComponentToComponent SkeletalMesh "hand_r" "SnapToTarget" "KeepWorld" "KeepRelative" true)
  (Collision|SetCollisionEnabled (Variables|Default|GetBox) "NoCollision"))

(event EventDrop
  (Transformation|DetachFromActor "KeepWorld" "KeepWorld" "KeepWorld")
  (Collision|SetCollisionEnabled (Variables|Default|GetBox) "QueryAndPhysics"))

(fn ConstructionScript)