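; BP_LoopsAndLists is a demo actor for loops and arrays that prints randomly colored debug messages.
; BeginPlay starts a self-calling event that counts iterations, waits a second, then calls PrintColors, repeating endlessly.
; PrintColors shuffles the color array and loops over it, but prints a random pick instead of the loop element.
; The pure Random node re-evaluates per use, so printed index and color can differ.
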(event Custom|Delay%20loop
  (Development|PrintString (Utilities|String|Append "Starting Delay Loop #" (Utilities|String|ToString(Integer) (Variables|Default|GetDelayLoopCounter))))
  (Math|Integer|IncrementInt (Variables|Default|GetDelayLoopCounter)
    (:%20%20
      (Utilities|FlowControl|Delay 1.0)
      (CallFunction|PrintColors)
      (CallFunction|DelayLoop))))

(event Custom|Print%20Colors
  (bind _array (Utilities|Array|MakeArray "(R=1.000000,G=0.000528,B=0.043476,A=1.000000)" "(R=0.321656,G=1.000000,B=0.013734,A=1.000000)" "(R=0.000000,G=0.239394,B=1.000000,A=1.000000)" "(R=1.000000,G=0.810581,B=0.000326,A=1.000000)"))
  (bind _textcolors (Variables|Default|Gettextcolors))
  (bind (_outitem _outindex) (Utilities|Array|Random _array))
  (Utilities|Array|Shuffle _textcolors)
  (for _array_element _textcolors
    (Development|PrintString (Utilities|String|Append "Printing Color #" (Utilities|String|ToString(Integer) _outindex)) true true _outitem))
  (Development|PrintString "We are Done Printing Colors!!!" true true "(R=0.000000,G=0.000000,B=0.000000,A=1.000000)"))

(event EventBeginPlay
  (Development|PrintString "Loops and lists is active.")
  (CallFunction|DelayLoop) ; Start the delay loop
)

(fn ConstructionScript)