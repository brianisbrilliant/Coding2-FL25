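; Demo actor that prints messages to show how different Blueprint loop types and color arrays behave.
; BeginPlay starts DelayLoop, a self-calling event that prints its run count, waits a second, then passes a DoN gate capped at twenty to run a ForLoop.
; The ForLoop prints indices in colors from an inline array.
; While (countdown with a Delay inside) and ForEach variants exist, but their calls are disconnected from execution.
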(event Custom|DelayLoop
  (Development|PrintText (Utilities|Text|FormatText "This has run {count} times." (stale _counter)))
  (Utilities|FlowControl|Delay 1.0)
  (bind _counter (Utilities|FlowControl|DoN 20)
    (:Exit
      (CallFunction|StartforLoop)
      (CallFunction|DelayLoop) ; Restart The Loop
    )))

(event Custom|StartForLoop
  (bind _array (Utilities|Array|MakeArray "(R=0.556207,G=0.003916,B=1.000000,A=1.000000)" "(R=1.000000,G=0.000000,B=0.030010,A=1.000000)" "(R=1.000000,G=0.819462,B=0.002650,A=1.000000)" "(R=0.000000,G=0.894369,B=1.000000,A=1.000000)" "(R=1.000000,G=0.335624,B=0.000000,A=1.000000)" "(R=0.119349,G=0.000000,B=1.000000,A=1.000000)"))
  (for _index (range 0 (- (Utilities|Array|Length _array) 1) 2)
    (Development|PrintText (Utilities|Text|FormatText "This is Index #{index}." _index) true true (Utilities|Array|Get(acopy) _array _index))))

(event Custom|StartWhileLoop
  (while (> (Variables|Default|GetWhileLoopCounter) 0) ; Sentinal loop is a while(true) loop
    (Development|PrintText (Utilities|Text|FormatText "There are {count} more uses in this loop." (Variables|Default|GetWhileLoopCounter)) true true "(R=1.000000,G=0.005854,B=0.632989,A=1.000000)")
    (Math|Integer|DecrementInt (Variables|Default|GetWhileLoopCounter) ; Decrement Int
      (:%20%20
        (Utilities|FlowControl|Delay 0.2)
        (Development|PrintText "after delay" true true "(R=1.000000,G=0.819729,B=0.000000,A=1.000000)"))))
  (Variables|Default|SetWhileLoopCounter 10))

(event Custom|StartForeachLoop
  (for (_array_element _array_index) (Utilities|Array|MakeArray "(R=0.556207,G=0.003916,B=1.000000,A=1.000000)" "(R=1.000000,G=0.000000,B=0.030010,A=1.000000)" "(R=1.000000,G=0.819462,B=0.002650,A=1.000000)" "(R=0.000000,G=0.894369,B=1.000000,A=1.000000)" "(R=1.000000,G=0.335624,B=0.000000,A=1.000000)" "(R=0.119349,G=0.000000,B=1.000000,A=1.000000)")
    (Development|PrintText (Utilities|Text|FormatText "This is Index #{index}." _array_index) true true _array_element)))

(event EventBeginPlay
  (Development|PrintString "Loops and Lists BP Exists")
  (CallFunction|DelayLoop))

(fn ConstructionScript)