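; Machine gun weapon that the player can pick up, drop and fire in three-round bursts.
; Pickup attaches it to the hand_r socket of the given skeletal mesh and disables Box collision, while Drop detaches it and restores collision.
; UsePrimary spawns BP_PlayerBullet at the Scene component, aimed along camera rotation, repeating through a delayed loop while a Burst flag blocks re-triggering.
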(event EventDrop
  (Transformation|DetachFromActor "KeepWorld" "KeepWorld" "KeepWorld")
  (Collision|SetCollisionEnabled (Variables|Default|GetBox) "QueryAndPhysics"))

(event EventBeginPlay
  (Variables|Default|SetBurst false)
  (Variables|Default|SetburstCount 0))

(event EventPickup
  (params (SkeletalMesh :type Skeletal%20Mesh%20Component%20Object%20Reference))
  ;[0.15 0.15 0.15 0.5] Pickup Function
  (Transformation|AttachComponentToComponent SkeletalMesh "hand_r" "SnapToTarget" "SnapToTarget" "KeepRelative" true)
  (Collision|SetCollisionEnabled (Variables|Default|GetBox) "NoCollision"))

(event EventUsePrimary
  (if (not (Variables|Default|GetBurst))
    (Variables|Default|SetBurst true)
    (Game|SpawnActorfromClass "/Game/Blueprints/BP_PlayerBullet.BP_PlayerBullet_C" (Math|Transform|MakeTransform (Transformation|GetWorldLocation (Variables|Default|GetScene)) (Transformation|GetActorRotation (Game|GetPlayerCameraManager 0)) "1.000000,1.000000,1.000000") "Undefined" "MultiplyWithRoot" 0 0 :!label _label)
    (Math|Integer|IncrementInt (Variables|Default|GetburstCount)
      (:%20%20
        (if (< (Variables|Default|GetburstCount) 3)
          (Utilities|FlowControl|Delay 0.2)
          (Development|PrintString "shooting")
          (goto _label)
          (else
            (Variables|Default|SetburstCount 0)
            (Variables|Default|SetBurst false)
            (Development|PrintString "burst finished")))))))

(fn ConstructionScript)