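; Player bullet actor that flies forward and damages actors tagged Enemy.
; Tick moves it a fixed step along its forward vector with sweep, unscaled by delta time.
; BeginPlay starts a delayed self-destroy and plays a gunshot sound at the world origin.
; Sphere overlap sends flat damage to enemies through EDamageMessage, without destroying the bullet on hit.
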(event OnComponentBeginOverlap(Sphere)
  (params (OverlappedComponent :type Primitive%20Component%20Object%20Reference) (OtherActor :type Actor%20Object%20Reference) (OtherComp :type Primitive%20Component%20Object%20Reference) (OtherBodyIndex :type Integer) (bFromSweep :type Boolean) (SweepResult :type Hit%20Result%20Structure%20%28by%20ref%29))
  (if (Actor|ActorHasTag OtherActor "Enemy")
    (Class|BPIDamage|EDamage(Message) OtherActor 35.0)))

(event Custom|Destroy
  (Utilities|FlowControl|Delay 1e+01)
  (Actor|DestroyActor))

(event EventTick
  (params (DeltaSeconds :type Float%20%28single-precision%29))
  (Transformation|SetActorLocation (+ (Transformation|GetActorLocation) (* (Transformation|GetActorForwardVector) 1e+01)) true false))

(event EventBeginPlay
  (CallFunction|Destroy)
  (Audio|SpawnSoundatLocation "/Game/Sound/mixkit-game-gun-shot-1662.mixkit-game-gun-shot-1662" "0, 0, 0" "0, 0, 0" 1.0 1.0 0.0 0 0))

(fn ConstructionScript)