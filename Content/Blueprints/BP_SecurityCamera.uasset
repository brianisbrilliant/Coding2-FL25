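; Security camera actor that alerts nearby enemies when the player character enters its cone.
; On the cone's begin overlap, it runs a multi-sphere trace on the Camera channel around its own location.
; Each hit actor tagged Enemy receives an AlertMessage with the player's location.
; The alert sound plays at the camera once per Enemy hit, so it stays silent when none are found.
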(event OnComponentBeginOverlap(Cone)
  (params (OverlappedComponent :type Primitive%20Component%20Object%20Reference) (OtherActor :type Actor%20Object%20Reference) (OtherComp :type Primitive%20Component%20Object%20Reference) (OtherBodyIndex :type Integer) (bFromSweep :type Boolean) (SweepResult :type Hit%20Result%20Structure%20%28by%20ref%29))
  (bind _returnvalue (Transformation|GetActorLocation))
  (if (== OtherActor (Game|GetPlayerCharacter 0))
    (bind (_outhits _returnvalue_2) (Collision|MultiSphereTraceByChannel _returnvalue _returnvalue 1e+03 "TraceTypeQuery2" false 0 "None"))
    (if _returnvalue_2
      (for _array_element _outhits
        (if (Actor|ActorHasTag (.hitactor _array_element) "Enemy")
          (Audio|PlaySoundatLocation "/Game/Sound/lego-city-hey-made-with-Voicemod.lego-city-hey-made-with-Voicemod" (Transformation|GetActorLocation) "0, 0, 0" 1.0 1.0 0.0 0 0 0 0)
          (Class|Enemy|Alert(Message) (.hitactor _array_element) (Transformation|GetActorLocation (Game|GetPlayerCharacter 0))))))))

(fn ConstructionScript)