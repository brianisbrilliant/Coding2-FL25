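; Turret actor that tracks and fires at the player while they are inside its detection sphere.
; Sphere overlap events set a shooting flag for the player character, and Tick uses it to turn the turret's yaw toward them.
; A self-looping Shooting event spawns BP_Bullet at the shooting point, aimed at the player, then repeats after a short delay until the flag clears.
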(event OnComponentBeginOverlap(Sphere)
  (params (OverlappedComponent :type Primitive%20Component%20Object%20Reference) (OtherActor :type Actor%20Object%20Reference) (OtherComp :type Primitive%20Component%20Object%20Reference) (OtherBodyIndex :type Integer) (bFromSweep :type Boolean) (SweepResult :type Hit%20Result%20Structure%20%28by%20ref%29))
  (if (== OtherActor (Game|GetPlayerCharacter 0))
    (Variables|Default|SetIsShooting true)
    (CallFunction|Shooting)))

(event OnComponentEndOverlap(Sphere)
  (params (OverlappedComponent :type Primitive%20Component%20Object%20Reference) (OtherActor :type Actor%20Object%20Reference) (OtherComp :type Primitive%20Component%20Object%20Reference) (OtherBodyIndex :type Integer))
  (if (== OtherActor (Game|GetPlayerCharacter 0))
    (Variables|Default|SetIsShooting false)))

(event Custom|Shooting
  (bind _shootingpoint (Variables|Default|GetShootingPoint))
  (bind _returnvalue (Transformation|GetWorldLocation _shootingpoint))
  (if (Variables|Default|GetIsShooting) :!label _label
    (Game|SpawnActorfromClass "/Game/Blueprints/BP_Bullet.BP_Bullet_C" (Math|Transform|MakeTransform _returnvalue (Math|Rotator|FindLookatRotation _returnvalue (Transformation|GetActorLocation (Game|GetPlayerCharacter 0))) "1.000000,1.000000,1.000000") "Undefined" "MultiplyWithRoot" 0 0)
    (Utilities|FlowControl|Delay 1.0)
    (goto _label)))

(event EventTick
  (params (DeltaSeconds :type Float%20%28single-precision%29))
  (if (Variables|Default|GetIsShooting)
    (Transformation|SetActorRotation (Math|Rotator|MakeRotator 0.0 0.0 (.yaw (Math|Rotator|FindLookatRotation (Transformation|GetWorldLocation (Variables|Default|GetShootingPoint)) (Transformation|GetActorLocation (Game|GetPlayerCharacter 0))))))))

(fn ConstructionScript)